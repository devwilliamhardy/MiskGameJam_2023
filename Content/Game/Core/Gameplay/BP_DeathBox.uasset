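; BP_DeathBox is a kill volume that sends the player back to the start of the level when they overlap its box.
; It stops their movement and the "gameSpline" designated path's following, then teleports them high above the PlayerStart.
; It resets that path's move loop, all obstacles and all platform managers.
; After a short retriggerable delay it increments the GameState death count and calls its death event.
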(event OnComponentBeginOverlap(Box)
  (params (OverlappedComponent :type Primitive%20Component%20Object%20Reference) (OtherActor :type Actor%20Object%20Reference) (OtherComp :type Primitive%20Component%20Object%20Reference) (OtherBodyIndex :type Integer) (bFromSweep :type Boolean) (SweepResult :type Hit%20Result%20Structure%20%28by%20ref%29))
  ;[1 1 1] Spawn player at initial spline point
  (bind _asbp_player_character (Utilities|Casting|CastToBP_PlayerCharacter OtherActor))
  (AI|Navigation|StopMovement (Pawn|GetController _asbp_player_character))
  (Components|Movement|StopMovementImmediately (Variables|/Script/Engine.Character|GetCharacterMovement _asbp_player_character))
  (bind _outactors (Actor|GetAllActorsOfClasswithTag "/Game/Game/Core/Gameplay/BP_DesignatedPath.BP_DesignatedPath_C" "gameSpline"))
  (Variables|/Game/Game/Core/Gameplay/BP_DesignatedPath.BP_DesignatedPath_C|SetbContinueFollowing (Utilities|Array|Get(acopy) _outactors) false)
  (bind _returnvalue (Actor|GetActorOfClass "/Script/Engine.PlayerStart"))
  (Transformation|Teleport _asbp_player_character (+ (.location (Transformation|GetActorTransform _returnvalue)) "0.000000,0.000000,1000.000000") (.rotation (Transformation|GetActorTransform _returnvalue)))
  (if true
    (Default|ResetMoveLoop (Utilities|Array|Get(acopy) _outactors))
    (bind _outactors_2 (Actor|GetAllActorsOfClass "/Game/Game/Core/Gameplay/Obstacles/BP_Obstacle_Master.BP_Obstacle_Master_C"))
    (for _array_element _outactors_2
      (Default|CallOnGameRestart _array_element))
    (bind _outactors_3 (Actor|GetAllActorsOfClass "/Game/Game/Core/Gameplay/BP_PlatformManager.BP_PlatformManager_C"))
    (for _array_element_2 _outactors_3
      (Default|ResetActor _array_element_2))
    (bind _asbp_game_state (Utilities|Casting|CastToBP_GameState (Game|GetGameState)))
    (Utilities|FlowControl|RetriggerableDelay 0.2)
    (Math|Integer|IncrementInt (Variables|/Game/Game/Core/Engine/BP_GameState.BP_GameState_C|GetDeaths _asbp_game_state)
      (:%20%20
        (Default|CallOnDeath _asbp_game_state)))))

(event EventBeginPlay)

(event Collision|EventActorBeginOverlap
  (params (OtherActor :type Actor%20Object%20Reference)))

(event EventTick
  (params (DeltaSeconds :type Float%20%28single-precision%29)))

(fn ConstructionScript)