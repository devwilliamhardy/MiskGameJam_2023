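; BP_DesignatedPath is a spline actor that walks an AI-controlled character along its points for menu and gameplay sequences.
; It async-loads a connected path to reuse its character, or async-loads a class to spawn one at the first point and make it the view target.
; Menu paths move immediately and teleport the character to the spline's end on game start, while others start moving then.
; Movement chains AI MoveTo calls per point; construction adds a start arrow and an optional end-game child actor.
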(event Custom|ResetMoveLoop
  ;[1 1 1] Reset loop movement
  (Variables|Default|SetbContinueFollowing true)
  (Variables|Default|SetCurrentSplinePointIndex 0)
  (Utilities|MovePlayerAlongSpline))

(event Custom|OnGameStarted_Event
  (bind _path (Variables|Default|GetPath))
  ;[1 1 1] Spawn character
  (if (Variables|Default|GetbIsMenu)
    (Transformation|Teleport (Variables|Default|GetCharacterRef) (Spline|GetLocationatDistanceAlongSpline _path (Spline|GetSplineLength _path) "World") "0, 0, 0")
    (else
      (Utilities|MovePlayerAlongSpline))))

(event EventBeginPlay
  (bind _path (Variables|Default|GetPath))
  (bind _returnvalue (Spline|GetTransformatSplinePoint _path 0 "World" false))
  ;[1 1 1] Spawn character
  (bind _connectedpath (Variables|Default|GetConnectedPath)
    (:then
      (bind _object (Utilities|AsyncLoadAsset _connectedpath)
        (:Completed
          (bind _asbp_designated_path (Utilities|Casting|CastToBP_DesignatedPath _object))
          (Variables|Default|SetCharacterRef (Variables|BP_DesignatedPath_C|GetCharacterRef _asbp_designated_path)))))
    (:else
      (bind _class (Utilities|AsyncLoadClassAsset (Variables|Default|GetCharacterClass))
        (:Completed
          (bind _aspawn (Utilities|Casting|CastToPawnClass _class))
          (bind _returnvalue_2 (AI|SpawnAIFromClass _aspawn 0 (.location _returnvalue) (.rotation _returnvalue) true 0))
          (bind _output_get (Variables|Default|SetCharacterRef _returnvalue_2))
          (Game|Player|SetViewTargetwithBlend (Game|GetPlayerController 0) _output_get 0.0 "VTBlend_Linear" 0.0 false)))))
  (bind _asbp_game_instance (Utilities|Casting|CastToBP_GameInstance (Game|GetGameInstance)))
  (EventDispatchers|BindEventtoOnGameStarted _asbp_game_instance (delegate Custom|OnGameStarted_Event))
  (if (Variables|Default|GetbIsMenu)
    (Utilities|MovePlayerAlongSpline)))

(fn ConstructionScript
  (bind _path (Variables|Default|GetPath))
  (bind _returnvalue (Spline|GetNumberOfSplinePoints _path))
  (bind _returnvalue_2 (- _returnvalue 1))
  (bind _returnvalue_3 (Spline|GetTransformatSplinePoint _path _returnvalue_2 "Local" false))
  (AddComponent|AddArrowComponent false (Spline|GetTransformatSplinePoint _path 0 "Local" false))
  (if (Variables|Default|GetbEndGame)
    (AddComponent|AddChildActorComponent false (Math|Transform|MakeTransform (.location _returnvalue_3) (.rotation _returnvalue_3) "1.000000,1.000000,1.000000"))))