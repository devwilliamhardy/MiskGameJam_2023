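; BP_PlatformManager spawns a row of falling floors and drops them in random order once the player arrives.
; The construction script adds evenly spaced BP_FallingFloor child actors along local X and records their references.
; Player overlap with PlayerDetector starts a looping one-second timer that activates and removes random floors from a working list, stopping when none is valid.
; ResetActor rebuilds both lists with newly added floors, without destroying the old ones.
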(event OnComponentBeginOverlap(PlayerDetector)
  (params (OverlappedComponent :type Primitive%20Component%20Object%20Reference) (OtherActor :type Actor%20Object%20Reference) (OtherComp :type Primitive%20Component%20Object%20Reference) (OtherBodyIndex :type Integer) (bFromSweep :type Boolean) (SweepResult :type Hit%20Result%20Structure%20%28by%20ref%29))
  (Utilities|Casting|CastToBP_PlayerCharacter OtherActor)
  (Utilities|Time|SetTimerbyFunctionName 0 "RandomDropTimer" 1.0 true))

(event Custom|ResetActor
  (Variables|Default|SetResetValue (Utilities|Array|LastIndex (Variables|Default|GetFallingFloorRef)))
  (Utilities|Array|Clear (Variables|Default|GetFallingFloorRef))
  (for _index (range 0 (Variables|Default|GetResetValue))
    (bind _returnvalue (AddComponent|AddChildActorComponent false (Math|Transform|MakeTransform (Math|Vector|MakeVector (Math|Conversions|ToFloat(Integer) (* _index 250)) 0.0 0.0))))
    (bind _asbp_falling_floor (Utilities|Casting|CastToBP_FallingFloor (Variables|/Script/Engine.ChildActorComponent|GetChildActor _returnvalue)))
    (Utilities|Array|Add (Variables|Default|GetFallingFloorRef) _asbp_falling_floor))
  (Variables|Default|SetCurrentFallingFloorRef (Variables|Default|GetFallingFloorRef)))

(event EventBeginPlay
  (Variables|Default|SetCurrentFallingFloorRef (Variables|Default|GetFallingFloorRef)))

(fn ConstructionScript
  (for _index (range 0 (- (Variables|Default|GetNumPlatforms) 1))
    (bind _returnvalue (AddComponent|AddChildActorComponent false (Math|Transform|MakeTransform (Math|Vector|MakeVector (Math|Conversions|ToFloat(Integer) (* _index 250)) 0.0 0.0))))
    (bind _asbp_falling_floor (Utilities|Casting|CastToBP_FallingFloor (Variables|/Script/Engine.ChildActorComponent|GetChildActor _returnvalue)))
    (Utilities|Array|Add (Variables|Default|GetFallingFloorRef) _asbp_falling_floor)))

(fn RandomDropTimer
  (bind _currentfallingfloorref (Variables|Default|GetCurrentFallingFloorRef))
  (bind _outitem (Utilities|Array|Random _currentfallingfloorref))
  (Utilities|IsValid _outitem
    (:Is%20Valid
      (bind _output_get (LocalVariables|SetChosenFloor _outitem))
      (Default|ActivateFloor _output_get)
      (Utilities|Array|RemoveItem (Variables|Default|GetCurrentFallingFloorRef) (LocalVariables|GetChosenFloor)))
    (:Is%20Not%20Valid
      (Utilities|Time|ClearTimerbyFunctionName 0 "RandomDropTimer"))))