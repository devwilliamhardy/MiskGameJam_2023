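; Base Blueprint for gameplay obstacles that responds to mouse hover and dragging.
; BeginPlay binds drag, game restart and actor cursor events, with the MouseDetection component feeding the same hover and click logic.
; Hover and click swap the player's cursor between default, grab and closed-hand icons, while click and release broadcast drag start and end.
; The drag and restart handlers are empty stubs in this class.
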(event OnBeginCursorOver(MouseDetection)
  (params (TouchedComponent :type Primitive%20Component%20Object%20Reference))
  ;[1 1 1] Ignore the cluster fuck I'm stressed.
  (Variables|/Script/Engine.PlayerController|SetCurrentMouseCursor (Game|GetPlayerController 0) "GrabHand"))

(event OnClicked(MouseDetection)
  (params (TouchedComponent :type Primitive%20Component%20Object%20Reference) (ButtonPressed :type Key%20Structure :default "None"))
  ;[1 1 1] Ignore the cluster fuck I'm stressed.
  ;;[1 1 1] Mouse detection
  (Default|CallOnStartDragging)
  (Variables|/Script/Engine.PlayerController|SetCurrentMouseCursor (Game|GetPlayerController 0) "GrabHandClosed"))

(event OnReleased(MouseDetection)
  (params (TouchedComponent :type Primitive%20Component%20Object%20Reference) (ButtonReleased :type Key%20Structure :default "None"))
  ;[1 1 1] Ignore the cluster fuck I'm stressed.
  ;;[1 1 1] Mouse detection
  (Default|CallOnEndDragging))

(event OnEndCursorOver(MouseDetection)
  (params (TouchedComponent :type Primitive%20Component%20Object%20Reference))
  ;[1 1 1] Ignore the cluster fuck I'm stressed.
  (Variables|/Script/Engine.PlayerController|SetCurrentMouseCursor (Game|GetPlayerController 0) "Default"))

(event Custom|HandleMouseDragStart
  ;[1 1 1] Ignore the cluster fuck I'm stressed.
  ;;[1 1 1] Bind delegates
)

(event Custom|HandleMouseDragEnd
  ;[1 1 1] Ignore the cluster fuck I'm stressed.
  ;;[1 1 1] Bind delegates
)

(event Custom|OnGameRestart_Event
  ;[1 1 1] Ignore the cluster fuck I'm stressed.
  ;;[1 1 1] Bind delegates
)

(event Custom|OnBeginCursorOver_Event
  (params (TouchedActor :type Actor%20Object%20Reference))
  ;[1 1 1] Ignore the cluster fuck I'm stressed.
  (Variables|/Script/Engine.PlayerController|SetCurrentMouseCursor (Game|GetPlayerController 0) "GrabHand"))

(event Custom|OnEndCursorOver_Event
  (params (TouchedActor :type Actor%20Object%20Reference))
  ;[1 1 1] Ignore the cluster fuck I'm stressed.
  (Variables|/Script/Engine.PlayerController|SetCurrentMouseCursor (Game|GetPlayerController 0) "Default"))

(event Custom|OnClicked_Event
  (params (TouchedActor :type Actor%20Object%20Reference) (ButtonPressed :type Key%20Structure :default "None"))
  ;[1 1 1] Ignore the cluster fuck I'm stressed.
  ;;[1 1 1] Mouse detection
  (Default|CallOnStartDragging)
  (Variables|/Script/Engine.PlayerController|SetCurrentMouseCursor (Game|GetPlayerController 0) "GrabHandClosed"))

(event Custom|OnReleased_Event
  (params (TouchedActor :type Actor%20Object%20Reference) (ButtonReleased :type Key%20Structure :default "None"))
  ;[1 1 1] Ignore the cluster fuck I'm stressed.
  ;;[1 1 1] Mouse detection
  (Default|CallOnEndDragging))

(event EventBeginPlay
  ;[1 1 1] Ignore the cluster fuck I'm stressed.
  ;;[1 1 1] Bind delegates
  (EventDispatchers|BindEventtoOnStartDragging (delegate Custom|HandleMouseDragStart))
  (EventDispatchers|BindEventtoOnEndDragging (delegate Custom|HandleMouseDragEnd))
  (EventDispatchers|BindEventtoOnGameRestart (delegate Custom|OnGameRestart_Event))
  (EventDispatchers|BindEventtoOnBeginCursorOver (delegate Custom|OnBeginCursorOver_Event))
  (EventDispatchers|BindEventtoOnEndCursorOver (delegate Custom|OnEndCursorOver_Event))
  (EventDispatchers|BindEventtoOnClicked (delegate Custom|OnClicked_Event))
  (EventDispatchers|BindEventtoOnReleased (delegate Custom|OnReleased_Event)))

(fn ConstructionScript)