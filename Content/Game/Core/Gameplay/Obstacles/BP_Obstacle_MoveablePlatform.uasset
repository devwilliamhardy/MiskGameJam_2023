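; Moveable platform obstacle that the player drags with the mouse along a single axis selected by Direction, returning to its starting transform on game restart.
; Drag start stores the grab offset and runs a looping timer that repositions the platform until drag end.
; Each update intersects a deprojected cursor line with a horizontal plane at the actor's height, keeping only the selected axis component, so the Z option yields no cursor-driven height.
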(event EventBeginPlay
  (|CallParentFunction)
  (Variables|Default|SetInitiialTransform (Transformation|GetActorTransform)))

(event EventOnGameRestartEvent
  (Transformation|SetActorTransform (Variables|Default|GetInitiialTransform) false true))

(event EventHandleMouseDragEnd
  ;[1 1 1] On drag end
  (Utilities|Time|ClearTimerbyFunctionName 0 "UpdatePlatformPosition"))

(event EventHandleMouseDragStart
  ;[1 1 1] On drag start
  (Variables|Default|SetMouseOffset (- (Transformation|GetActorLocation) (CallFunction|CalculateIntersectionPoit)))
  (Utilities|Time|SetTimerbyFunctionName 0 "UpdatePlatformPosition" 0.01 true))

(fn ConstructionScript
  (|CallParentFunction))

(fn UpdatePlatformPosition
  (Transformation|SetActorLocation (+ (CallFunction|CalculateIntersectionPoit) (Variables|Default|GetMouseOffset)) false false))

(fn CalculateIntersectionPoit
  (bind _returnvalue (Game|GetPlayerController 0))
  (bind _returnvalue_2 (Transformation|GetActorLocation))
  (bind _returnvalue_3 (Transformation|GetActorLocation))
  (bind _returnvalue_4 (Game|GetPlayerCameraManager 0))
  (bind (_locationx _locationy) (Class|WidgetLayoutLibrary|GetMousePositionScaledbyDPI _returnvalue))
  (bind _returnvalue_5 (Transformation|GetActorForwardVector _returnvalue_4))
  (bind (_worldposition _worlddirection) (Class|GameplayStatics|DeprojectScreentoWorld _returnvalue (Math|Vector2D|MakeVector2D _locationx _locationy)))
  (bind _returnvalue_6 (* _worlddirection 1e+04))
  (bind _returnvalue_7 (+ _returnvalue_5 _returnvalue_6))
  (bind _intersection (Class|KismetMathLibrary|LinePlaneIntersectionOriginNormal _worldposition _returnvalue_7 _returnvalue_2 "0.000000,0.000000,1.000000"))
  (bind (_x _y _z) (Math|Vector|BreakVector _intersection))
  (return (Utilities|Select :Index (Variables|Default|GetDirection) :NewEnumerator0 (Math|Vector|MakeVector _x (.y _returnvalue_3) (.z _returnvalue_3)) :NewEnumerator1 (Math|Vector|MakeVector (.x _returnvalue_3) _y (.z _returnvalue_3)) :NewEnumerator2 (Math|Vector|MakeVector (.x _returnvalue_3) (.y _returnvalue_3) _z))))