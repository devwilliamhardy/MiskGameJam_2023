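; Shape-filler obstacle that cycles a random, non-repeating mesh on a timer, with a timeline-driven scale transition.
; A mouse drag start stops the cycling and restores full scale.
; Player overlap also stops it, drops the shape by the DropPoint spline's length, and shrinks it away if it mismatches IntendedShape.
; Game restart resets it, and construction places a debug mesh at the spline's end.
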(event OnComponentBeginOverlap(PlayerDetector)
  (params (OverlappedComponent :type Primitive%20Component%20Object%20Reference) (OtherActor :type Actor%20Object%20Reference) (OtherComp :type Primitive%20Component%20Object%20Reference) (OtherBodyIndex :type Integer) (bFromSweep :type Boolean) (SweepResult :type Hit%20Result%20Structure%20%28by%20ref%29))
  ;[1 1 1] Player in range drop shape
  (Utilities|Casting|CastToBP_PlayerCharacter OtherActor)
  (Utilities|FlowControl|DoOnce false
    (:Completed
      (Utilities|Time|ClearTimerbyFunctionName 0 "ChooseRandomShape")
      (CallFunction|ResetScale)
      (Utilities|FlowControl|Sequence
        (:then_0
          (bind _alpha (Timeline|TL_UpdateShapeTransform PlayFromStart)
            (:Update
              (Transformation|SetRelativeLocation (Variables|Default|GetSM_Shape) (Math|Vector|Lerp(Vector) "0, 0, 0" (Math|Vector|MakeVector 0.0 0.0 (* (Spline|GetSplineLength (Variables|Default|GetDropPoint)) -1.0)) _alpha) false false))))
        (:then_1
          (if (not (== (Variables|/Script/Engine.StaticMeshComponent|GetStaticMesh (Variables|Default|GetSM_Shape)) (Utilities|Select :Index (Variables|Default|GetIntendedShape) :NewEnumerator0 "/Game/Game/Art/Enviornment/Cube_Shape.Cube_Shape" :NewEnumerator1 "/Game/Game/Art/Enviornment/Ball_Shape.Ball_Shape" :NewEnumerator2 "/Game/Game/Art/Enviornment/Pyramid_Shape.Pyramid_Shape")))
            (bind _alpha_2 (Timeline|TL_WrongShape PlayFromStart)
              (:Update
                (Transformation|SetRelativeScale3D (Variables|Default|GetSM_Shape) (Math|Vector|Lerp(Vector) "1.000000,1.000000,1.000000" "0, 0, 0" _alpha_2))))))))))

(event Custom|ChooseRandomShape
  ;[1 1 1] Change shape, transition
  (Components|StaticMesh|SetStaticMesh (Variables|Default|GetSM_Shape) (CallFunction|FindRandomShape))
  (Components|Timeline|SetPlayRate (Variables|Default|GetTL_ShapeChange) (/ 1.0 (Variables|Default|GetShapeChangeDelay)))
  (bind _alpha (Timeline|TL_ShapeChange PlayFromStart)
    (:Update
      (Transformation|SetRelativeScale3D (Variables|Default|GetSM_Shape) (Math|Conversions|ToVector(Float) _alpha)))))

(event Custom|ResetScale
  ;[1 1 1] Resets scale back to 1.0f
  (Audio|Components|Audio|Stop (Variables|Default|GetTL_ShapeChange))
  (bind _alpha (Timeline|TL_ScaleUp PlayFromStart)
    (:Update
      (Transformation|SetRelativeScale3D (Variables|Default|GetSM_Shape) (Math|Vector|Lerp(Vector) (Variables|/Script/Engine.SceneComponent|GetRelativeScale3D (Variables|Default|GetSM_Shape)) "1.000000,1.000000,1.000000" _alpha)))))

(event EventBeginPlay
  ;[1 1 1] Update shape
  (|CallParentFunction)
  (Utilities|Time|SetTimerbyFunctionName 0 "ChooseRandomShape" (Variables|Default|GetShapeChangeDelay) true))

(event EventOnGameRestartEvent
  (Audio|Components|Audio|Play (Variables|Default|GetTL_ShapeChange))
  (Utilities|Time|SetTimerbyFunctionName 0 "ChooseRandomShape" (Variables|Default|GetShapeChangeDelay) true)
  (Transformation|SetRelativeLocation (Variables|Default|GetSM_Shape) "0, 0, 0" false false)
  (Transformation|SetRelativeScale3D (Variables|Default|GetSM_Shape) "1.000000,1.000000,1.000000")
  ;[1 1 1] Player in range drop shape
  (Utilities|FlowControl|DoOnce false) ; enters at Reset
)

(event EventHandleMouseDragStart
  ;[1 1 1] On player clicked
  (Utilities|Time|ClearTimerbyFunctionName 0 "ChooseRandomShape")
  (CallFunction|ResetScale))

(fn ConstructionScript
  (bind _droppoint (Variables|Default|GetDropPoint))
  (|CallParentFunction)
  (Components|StaticMesh|SetStaticMesh (Variables|Default|GetStaticMesh) (Variables|Default|GetDebugMesh))
  (Transformation|SetWorldTransform (Variables|Default|GetStaticMesh) (Math|Transform|MakeTransform (.location (Spline|GetTransformatDistanceAlongSpline _droppoint (Spline|GetSplineLength _droppoint) "World" false)) "0, 0, 0" "1.000000,1.000000,1.000000") false false))

(fn FindRandomShape
  (bind _output_get (LocalVariables|SetTemporaryShapes (Variables|Default|GetPossibleShapes)))
  (Utilities|Array|RemoveItem _output_get (Variables|/Script/Engine.StaticMeshComponent|GetStaticMesh (Variables|Default|GetSM_Shape)))
  (return (.OutItem (Utilities|Array|Random (LocalVariables|GetTemporaryShapes)))))